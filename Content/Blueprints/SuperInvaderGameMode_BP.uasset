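; Game mode for Super Invader that runs the wave-by-wave round loop.
; RoundStart looks up a string-encoded layout for the current WaveCount in LevelMap and passes it to SpawnWave, which is not defined in this graph.
; RoundOver advances the wave and restarts on a win, or only prints a message on a loss.
; LevelMap hardcodes the first three layouts and returns an empty string beyond them.
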(event EventBeginPlay)

(event EventTick
  (params (DeltaSeconds :type Float%20%28single-precision%29)))

(event EventRoundStart
  (bind _newleveldata (CallFunction|LevelMap (Variables|Default|GetWaveCount)))
  (Class|SuperInvadersGameModeBase|SpawnWave _newleveldata))

(event EventRoundOver
  (params (PlayerWon :type Boolean))
  (if PlayerWon
    (Math|Integer|IncrementInt (Variables|Default|GetWaveCount)
      (:%20%20
        (Class|SuperInvadersGameModeBase|RoundStart)))
    (else
      (Development|PrintString "We died"))))

(fn ConstructionScript)

(fn LevelMap
  (params (LevelCount :type Integer))
  (Utilities|FlowControl|Sequence
    (:then_0
      (switch int LevelCount
        (:Default
          (LocalVariables|SetLevelData ""))
        (:0
          (LocalVariables|SetLevelData "w"))
        (:1
          (LocalVariables|SetLevelData "nnnnnnwnnnnnnw"))
        (:2
          (LocalVariables|SetLevelData "nnnnnnwnnnnnnwnnnnnnwnnnnn"))))
    (:then_1
      (return (LocalVariables|GetLevelData)))))